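; Elevator actor that smoothly moves to an extended position while the player overlaps it and returns to standby when the player leaves.
; Begin and end overlap events set a return flag, then share one timeline that lerps the actor toward the chosen position.
; Each trigger captures the current location and restarts the timeline, so reversing mid-travel starts from where the elevator is.
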(event Collision|EventActorBeginOverlap
  (params (OtherActor :type Actor%20Object%20Reference))
  ;[0.7656 0.05822 0.05822] Player Detection
  (if (== OtherActor (Game|GetPlayerCharacter 0)) ; Future: Add condition to check if stage completed
    (Variables|Default|SetReturnToStandbyPos false) ; False: Elevator extends
    ;[1 1 1] Move elevator! (to StandbyPos, up / ExtendedPos, down)
    (Variables|Default|SetStartingPos (Transformation|GetActorLocation)) ; Where is the platform right now?
    (bind _movementalpha (Timeline|Timeline PlayFromStart)
      (:Update
        (Transformation|SetActorLocation (Math|Vector|Lerp(Vector) (Variables|Default|GetStartingPos) (select (Variables|Default|GetReturnToStandbyPos) (Variables|Default|GetStandbyPos) (Variables|Default|GetExtendedPos)) _movementalpha) false false)))))

(event Collision|EventActorEndOverlap
  (params (OtherActor :type Actor%20Object%20Reference))
  ;[0.7656 0.05822 0.05822] Player Detection
  (if (== (Game|GetPlayerCharacter 0) OtherActor)
    (Variables|Default|SetReturnToStandbyPos true) ; True: Elevator returns to Standby
    ;[1 1 1] Move elevator! (to StandbyPos, up / ExtendedPos, down)
    (Variables|Default|SetStartingPos (Transformation|GetActorLocation)) ; Where is the platform right now?
    (bind _movementalpha (Timeline|Timeline PlayFromStart)
      (:Update
        (Transformation|SetActorLocation (Math|Vector|Lerp(Vector) (Variables|Default|GetStartingPos) (select (Variables|Default|GetReturnToStandbyPos) (Variables|Default|GetStandbyPos) (Variables|Default|GetExtendedPos)) _movementalpha) false false)))))

(fn ConstructionScript)