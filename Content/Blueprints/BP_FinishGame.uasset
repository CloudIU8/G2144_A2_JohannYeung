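; BP_FinishGame is a trigger actor that ends the game when the player character overlaps it.
; On BeginPlay it caches the player's BP_FirstPersonCharacter and the GM_KineticArtifact game mode.
; On overlap it checks that the other actor is that cached character, then calls FinishGame on the game mode, which handles the ending.
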(event EventBeginPlay
  ;[1 1 1] Get references
  (bind _asbp_first_person_character (Utilities|Casting|CastToBP_FirstPersonCharacter (Game|GetPlayerCharacter 0)))
  (Variables|Default|SetAs%20BP%20First%20Person%20Character _asbp_first_person_character)
  (bind _asgm_kinetic_artifact (Utilities|Casting|CastToGM_KineticArtifact (Game|GetGameMode)))
  (Variables|Default|SetAs%20GM%20Kinetic%20Artifact _asgm_kinetic_artifact))

(event Collision|EventActorBeginOverlap
  (params (OtherActor :type Actor%20Object%20Reference))
  (if (== OtherActor (Variables|Default|GetAs%20BP%20First%20Person%20Character))
    ;[0.4427 1 0.4624] Handle in Game Mode
    (Default|FinishGame (Variables|Default|GetAs%20GM%20Kinetic%20Artifact))))

(fn ConstructionScript)