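; Game mode for Curious Cabinet that tracks puzzle completion and unlocks the matching elevator.
; On BeginPlay it caches every BP_Elevator in the level.
; CheckPuzzle1Status counts active magic plates in a status map and calls PuzzleComplete once enough are active, printing debug messages along the way.
; PuzzleComplete enables the first cached elevator whose number matches the completed puzzle.
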(event Custom|PuzzleComplete
  (params (Puzzle%20Number :type Integer))
  ;[1 1 1] Enable elevator upon puzzle completion
  (bind _array_element (Utilities|Array|ForEachLoopwithBreak (Variables|Default|GetLevelElevators) :!label _label)
    (:LoopBody
      (if (== (Variables|/Game/Blueprints/BP_Elevator.BP_Elevator_C|GetElevatorNumber _array_element) Puzzle%20Number) ; Find elevator matching completed puzzle
        (Variables|/Game/Blueprints/BP_Elevator.BP_Elevator_C|SetElevatorEnabled _array_element true)
        (goto _label Break)))))

(event EventBeginPlay
  ;[1 0.2052 0.2052] Begin Play
  (Utilities|FlowControl|Sequence
    (:then_0
      ;[1 1 1] Get elevator references
      (bind _outactors (Actor|GetAllActorsOfClass "/Game/Blueprints/BP_Elevator.BP_Elevator_C"))
      (Variables|Default|SetLevelElevators _outactors))))

(fn ConstructionScript)

(fn CheckPuzzle1Status
  (Variables|Default|SetActivePlates 0)
  (bind _values (Utilities|Map|Values (Variables|Default|GetPuzzle1PlatesStatus)))
  (bind _array_element (Utilities|Array|ForEachLoopwithBreak _values) ; Loops through MagicPlates
    (:LoopBody
      ;[1 1 1] Checks each MagicPlate: Is activated?
      (if _array_element
        (bind _result (Math|Integer|IncrementInt (Variables|Default|GetActivePlates))
          (:%20%20
            (bind _output_get (Variables|Default|SetActivePlates _result))
            (Development|PrintString (Utilities|String|Append (Utilities|String|ToString(Integer) _output_get) " plates are active.") true true "(R=0.000000,G=0.660000,B=1.000000,A=1.000000)" 2.0 "Puzzle1Check")))))
    (:Completed
      ;[0.7715 1 0.7624] Puzzle completion
      (if (>= (Variables|Default|GetActivePlates) 3)
        (CallFunction|PuzzleComplete 1)
        (Development|PrintString "Puzzle1Complete!") ; Puzzle complete!
      ))))