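; BP_MusicalPodium is a numbered puzzle podium that plays a note pitched from its ID through a G Lydian scale array.
; Construction sets the label, pitch value and dynamic emissive material; playback shifts one sound by equal-temperament semitone math.
; Activation plays the note, then after a short timer lights the podium and sends its ID to GM_KineticArtifact for evaluation.
; PlayWithoutActivating gives melody playback a momentary timeline glow without evaluation, while DeactivatePodium clears the glow next tick.
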(event Custom|ActivatePodium
  (bind _notepitchvalue (Variables|Default|GetNotePitchValue))
  (bind _returnvalue (- _notepitchvalue 1.0))
  (bind _returnvalue_2 (* _returnvalue 2.0))
  (bind _returnvalue_3 (/ _returnvalue_2 12.0))
  (bind _returnvalue_4 (Math|Float|Power 2.0 _returnvalue_3))
  (Utilities|Time|SetTimerbyEvent (delegate Custom|Process) 0.2)
  (Development|PrintString (Utilities|String|ToString(Float) _returnvalue_4)) ; Show during\nreflection!
  ;[1 1 1] Play note SFX!
  (Audio|PlaySoundatLocation "/Game/Sound/PodiumNoteG_freesound_community-sol-101774_Modulated.PodiumNoteG_freesound_community-sol-101774_Modulated" (Transformation|GetActorLocation) "0, 0, 0" 0.6 _returnvalue_4 0.0 0 0 0 0))

(event Custom|DeactivatePodium
  ;[1 1 1] Feedback: Default state
  (Utilities|FlowControl|DelayUntilNextTick)
  (Rendering|Material|SetScalarParameterValue (Variables|Default|GetDMI_PodiumEmissive) "EmissiveStrength" 0.0 :!class /Script/Engine.MaterialInstanceDynamic))

(event Custom|Process
  ;[1 1 1] Feedback: Glow!
  (Rendering|Material|SetScalarParameterValue (Variables|Default|GetDMI_PodiumEmissive) "EmissiveStrength" 1.0 :!class /Script/Engine.MaterialInstanceDynamic)
  ;[1 1 1] Update GM
  (bind _asgm_kinetic_artifact (Utilities|Casting|CastToGM_KineticArtifact (Game|GetGameMode)))
  (Default|EvaluatePuzzle _asgm_kinetic_artifact (Variables|Default|GetPodiumNoteID)))

(event Custom|PlayWithoutActivating
  ;[1 1 1] Play note, separate from other systems! Called by GM when player triggers PlayMelody.
  (Utilities|FlowControl|Sequence
    (:then_0
      (bind _emissivealpha (Timeline|PodiumMomentaryGlowTimeline PlayFromStart)
        (:Update
          (Rendering|Material|SetScalarParameterValue (Variables|Default|GetDMI_PodiumEmissive) "EmissiveStrength" _emissivealpha :!class /Script/Engine.MaterialInstanceDynamic))))
    (:then_1
      ;[1 1 1] Play note SFX!
      (Audio|PlaySoundatLocation "/Game/Sound/PodiumNoteG_freesound_community-sol-101774_Modulated.PodiumNoteG_freesound_community-sol-101774_Modulated" (Transformation|GetActorLocation) "0, 0, 0" 0.6 (Math|Float|Power 2.0 (/ (* (- (Variables|Default|GetNotePitchValue) 1.0) 2.0) 12.0)) 0.0 0 0 0 0))))

(fn ConstructionScript
  (Rendering|Components|TextRender|SetText (Variables|Default|GetTR_PodiumNumber) (Utilities|Text|ToText(Integer) (Variables|Default|GetPodiumNoteID)))
  (Variables|Default|SetNotePitchValue (Utilities|Array|Get(acopy) (Variables|Default|GetGLydianScaleValues) (- (Variables|Default|GetPodiumNoteID) 1)))
  ;[1 1 1] Create DMI to vary Emissive Strength during gameplay
  (bind _returnvalue (Rendering|Material|CreateDynamicMaterialInstance (Variables|Default|GetSM_PodiumSpot) 0 "/Game/Materials/M_EmissiveWhite.M_EmissiveWhite" "None" :!class /Script/Engine.PrimitiveComponent))
  (bind _output_get (Variables|Default|SetDMI_PodiumEmissive _returnvalue))
  (Rendering|Material|SetScalarParameterValue _output_get "EmissiveStrength" 0.0 :!class /Script/Engine.MaterialInstanceDynamic) ; Initialise at 0 (idle state)
)