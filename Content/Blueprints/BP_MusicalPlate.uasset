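; BP_MusicalPlate is a puzzle pressure plate that plays a melody when the player steps on it.
; Overlap plays a click and starts a short timer; if still active, the plate chimes, glows and asks GM_KineticArtifact to play the melody matching its PlateID.
; Stepping off plays a release sound, restores the pulsing standby material and clears the GameMode's PlayingMelody flag to stop the melody.
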(event Custom|SetMaterial_Activated
  ;[0.55 1 0.5349] Plate Activation
  (Rendering|Material|SetMaterial (Variables|Default|GetSM_PressurePlate) 0 "/Game/Materials/M_EmissiveWhite.M_EmissiveWhite") ; Glow!
)

(event Custom|SetMaterial_Standby
  ;[1 0.6112 0.5933] Plate Standby
  (Rendering|Material|SetMaterial (Variables|Default|GetSM_PressurePlate) 0 "/Game/Materials/M_EmissivePulse.M_EmissivePulse") ; Pulse!
)

(event Custom|ActivatePlate
  ;[1 1 1] Activate Plate & Call GM
  (if (Variables|Default|GetPlateActive)
    (Audio|PlaySoundatLocation "/Game/Sound/MusicalPlateChime_F_5.MusicalPlateChime_F_5" (Transformation|GetActorLocation) "0, 0, 0" 0.6 1.0 0.0 0 0 0 0)
    (CallFunction|SetMaterialActivated)
    (Default|PlayMelody (Variables|Default|GetGame%20Mode%20Ref) (Variables|Default|GetPlateID)) ; Play the melody of the puzzle matching this plate's ID.
  ))

(event EventBeginPlay
  ;[1 1 1] Obtain GM reference
  (bind _asgm_kinetic_artifact (Utilities|Casting|CastToGM_KineticArtifact (Game|GetGameMode)))
  (Variables|Default|SetGame%20Mode%20Ref _asgm_kinetic_artifact))

(event EventInteractableActorIsOverlapped
  (params (Player%20Ref :type Actor%20Object%20Reference))
  ;[1 0.2677 0.2677] Activated by Player
  (Variables|Default|SetPlateActive true)
  ;[1 1 1] Feedback: Stepped on
  (Audio|PlaySoundatLocation "/Game/Sound/MagicPlateClick.MagicPlateClick" (Transformation|GetActorLocation) "0, 0, 0" 1.0 1.0 0.0 0 0 0 0)
  (Utilities|Time|SetTimerbyEvent (delegate Custom|ActivatePlate) 0.5))

(event EventInteractableActorEndOverlap
  (params (PlayerRef :type Actor%20Object%20Reference))
  ;[1 0.2677 0.2677] Deactivated by Player
  (Variables|Default|SetPlateActive false)
  ;[1 1 1] Feedback: Stepped off
  (Audio|PlaySoundatLocation "/Game/Sound/MagicPlateRelease.MagicPlateRelease" (Transformation|GetActorLocation) "0, 0, 0" 1.0 1.0 0.0 0 0 0 0)
  (CallFunction|SetMaterialStandby)
  ;[1 1 1] GM: Stop playing melody if currently running
  (Variables|/Game/Blueprints/GameModes/GM_KineticArtifact.GM_KineticArtifact_C|SetPlayingMelody (Variables|Default|GetGame%20Mode%20Ref) false))

(fn ConstructionScript)