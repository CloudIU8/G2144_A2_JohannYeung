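; BP_MagicPlate is a timed pressure plate for Puzzle 1 in the Curious Cabinet game mode.
; On overlap it marks its PlateID active in the GameMode's status map, swaps to an emissive material, plays sounds and triggers the puzzle check.
; A timer then restores the material and marks the plate inactive after ActivationTime.
; Leaving the plate only plays a release sound.
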(event Custom|DeactivatePlate
  ;[1 0.6601 0.674] Plate Deactivation
  (Rendering|Material|SetMaterial (Variables|Default|GetSM_PressurePlate) 0 "/Game/StarterContent/Materials/M_AssetPlatform.M_AssetPlatform")
  (Audio|PlaySoundatLocation "/Game/Sound/MagicPlateDeactivate.MagicPlateDeactivate" (Transformation|GetActorLocation) "0, 0, 0" 1.0 1.0 0.0 0 0 0 0)
  (Utilities|Map|Add (Variables|/Game/Blueprints/GameModes/GM_CuriousCabinet.GM_CuriousCabinet_C|GetPuzzle1PlatesStatus (Variables|Default|GetGM%20Curious%20Cabinet%20Ref)) (Variables|Default|GetPlateID) false) ; Updates plate activation status in GM
)

(event EventBeginPlay
  ;[1 1 1] Obtain GM reference
  (bind _asgm_curious_cabinet (Utilities|Casting|CastToGM_CuriousCabinet (Game|GetGameMode)))
  (Variables|Default|SetGM%20Curious%20Cabinet%20Ref _asgm_curious_cabinet))

(event EventInteractableActorIsOverlapped
  (params (Player%20Ref :type Actor%20Object%20Reference))
  (bind _sm_pressureplate (Variables|Default|GetSM_PressurePlate))
  (bind _returnvalue (Transformation|GetWorldLocation _sm_pressureplate))
  ;[1 1 1] Detect Player
  ;[0.55 1 0.5349] Plate Activation
  (Utilities|Map|Add (Variables|/Game/Blueprints/GameModes/GM_CuriousCabinet.GM_CuriousCabinet_C|GetPuzzle1PlatesStatus (Variables|Default|GetGM%20Curious%20Cabinet%20Ref)) (Variables|Default|GetPlateID) true) ; Updates plate activation status in GM
  (Rendering|Material|SetMaterial _sm_pressureplate 0 "/Game/Materials/M_EmissiveWhite.M_EmissiveWhite") ; Glow!
  (Audio|PlaySoundatLocation "/Game/Sound/MagicPlateClick.MagicPlateClick" _returnvalue "0, 0, 0" 1.0 1.0 0.0 0 0 0 0)
  (Audio|PlaySoundatLocation "/Game/Sound/MagicPlateActivate.MagicPlateActivate" _returnvalue "0, 0, 0" 0.6 1.0 0.0 0 0 0 0)
  (Default|CheckPuzzle1Status (Variables|Default|GetGM%20Curious%20Cabinet%20Ref))
  ;[1 0.6601 0.674] Plate Deactivation
  (Utilities|Time|SetTimerbyEvent (delegate Custom|DeactivatePlate) (Variables|Default|GetActivationTime)))

(event EventInteractableActorEndOverlap
  (params (PlayerRef :type Actor%20Object%20Reference))
  (Audio|PlaySoundatLocation "/Game/Sound/MagicPlateRelease.MagicPlateRelease" (Transformation|GetActorLocation) "0, 0, 0" 1.0 1.0 0.0 0 0 0 0))

(fn ConstructionScript)