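; BP_Puzzle2Cube is a puzzle cube that the player clicks to drop onto a podium.
; A player line trace hit enables physics on the mesh and plays a click sound.
; Hitting a BP_Puzzle2PodiumSpot activates that podium, freezes the cube and plays an impact sound.
; The construction script saves the starting location as the primed position, which PrimeForDrop uses to reset the cube with physics off.
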(event Collision|EventHit
  (params (MyComp :type Primitive%20Component%20Object%20Reference) (Other :type Actor%20Object%20Reference) (OtherComp :type Primitive%20Component%20Object%20Reference) (bSelfMoved :type Boolean) (HitLocation :type Vector :default "0, 0, 0") (HitNormal :type Vector :default "0, 0, 0") (NormalImpulse :type Vector :default "0, 0, 0") (Hit :type Hit%20Result%20Structure%20%28by%20ref%29))
  ;[1 0.151 0.151] Hit!
  ;[1 1 1] Check collision is with Podium
  (if (== (Utilities|GetClass Other) "/Game/Blueprints/BP_Puzzle2PodiumSpot.BP_Puzzle2PodiumSpot_C")
    (bind _asbp_puzzle_2podium_spot (Utilities|Casting|CastToBP_Puzzle2PodiumSpot Other))
    (Default|ActivatePodium _asbp_puzzle_2podium_spot)
    ;[1 1 1] Ensure cube is stationary
    (Physics|SetSimulatePhysics (Variables|Default|GetSM_Cube) false)
    ;[1 1 1] SFX
    (Audio|PlaySoundatLocation "/Game/Sound/CubeHitPodium.CubeHitPodium" (Transformation|GetActorLocation) "0, 0, 0" 3.0 1.0 0.3 0 0 0 0)))

(event EventPlayerLineTraceHit
  ;[1 0.2719 0.2719] Drop onto podium on player LMB
  (Physics|SetSimulatePhysics (Variables|Default|GetSM_Cube) true)
  ;[1 1 1] SFX
  (Audio|PlaySoundatLocation "/Game/Sound/CubeClicked.CubeClicked" (Transformation|GetActorLocation) "0, 0, 0" 0.8 1.0 0.0 0 0 0 0))

(fn ConstructionScript
  (Variables|Default|SetPrimedPosition (Transformation|GetActorLocation))
  (CallFunction|PrimeforDrop))

(fn PrimeforDrop
  (Physics|SetSimulatePhysics (Variables|Default|GetSM_Cube) false)
  (Transformation|SetWorldLocationAndRotation (Variables|Default|GetSM_Cube) (Variables|Default|GetPrimedPosition) "0, 0, 0" false false))