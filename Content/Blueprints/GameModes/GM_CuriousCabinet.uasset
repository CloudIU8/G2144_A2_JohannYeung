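; Game mode for the Curious Cabinet level that judges two puzzles, unlocks elevators and handles game completion.
; Puzzle 1 completes at three active plates; Puzzle 2 requires podiums activated in ascending order, resetting cubes and podiums on mistakes.
; PuzzleComplete uses a short timer to enable the cached BP_Elevator matching that puzzle number.
; FinishGame plays a win jingle and returns to the lobby map after a delay.
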(event Custom|FinishGame
  (Utilities|Time|SetTimerbyEvent (delegate Custom|ToMainMenu) 3.0)
  (Development|PrintString "Game complete! Loading main menu..." true true "(R=0.204660,G=0.619792,B=0.216095,A=1.000000)" 5.0 "LoadingMainMenu")
  ;[1 1 1] Win jingle SFX
  (Audio|PlaySoundatLocation "/Game/Sound/270545__littlerobotsoundfactory__jingle_win_01.270545__littlerobotsoundfactory__jingle_win_01" (Transformation|GetActorLocation (Game|GetPlayerCharacter 0)) "0, 0, 0" 1.0 1.0 0.0 0 0 0 0))

(event Custom|PuzzleComplete
  (params (Puzzle%20Number :type Integer))
  ;[1 1 1] Enable elevator upon puzzle completion
  (Utilities|Time|SetTimerbyEvent (delegate Custom|UnlockElevator) 0.5))

(event Custom|ToMainMenu
  (Game|OpenLevel(byObjectReference) "/Game/Levels/LobbyMap.LobbyMap"))

(event Custom|UnlockElevator
  ;[1 1 1] Enable elevator upon puzzle completion
  (bind _array_element (Utilities|Array|ForEachLoopwithBreak (Variables|Default|GetLevelElevators) :!label _label)
    (:LoopBody
      (if (== (Variables|/Game/Blueprints/BP_Elevator.BP_Elevator_C|GetElevatorNumber _array_element) (stale Custom|PuzzleComplete Puzzle%20Number)) ; Find elevator matching completed puzzle
        (Default|EnableElevator _array_element (stale Custom|PuzzleComplete Puzzle%20Number))
        (goto _label Break)))))

(event EventBeginPlay
  ;[1 0.2052 0.2052] Begin Play
  (Utilities|FlowControl|Sequence
    (:then_0
      ;[1 1 1] Get elevator references
      (bind _outactors (Actor|GetAllActorsOfClass "/Game/Blueprints/BP_Elevator.BP_Elevator_C"))
      (Variables|Default|SetLevelElevators _outactors))))

(fn ConstructionScript
  (bind _outactors (Actor|GetAllActorsOfClass "/Game/Blueprints/BP_Puzzle2PodiumSpot.BP_Puzzle2PodiumSpot_C"))
  (Variables|Default|SetTotalPodiums (Utilities|Array|Length _outactors)))

(fn CheckPuzzle1Status
  (Variables|Default|SetActivePlates 0)
  (bind _values (Utilities|Map|Values (Variables|Default|GetPuzzle1PlatesStatus)))
  (bind _array_element (Utilities|Array|ForEachLoopwithBreak _values) ; Loops through MagicPlates
    (:LoopBody
      ;[1 1 1] Checks each MagicPlate: Is activated?
      (if _array_element
        (bind _result (Math|Integer|IncrementInt (Variables|Default|GetActivePlates))
          (:%20%20
            (bind _output_get (Variables|Default|SetActivePlates _result))
            (Development|PrintString (Utilities|String|Append (Utilities|String|ToString(Integer) _output_get) " plates are active.") true true "(R=0.000000,G=0.660000,B=1.000000,A=1.000000)" 2.0 "Puzzle1Check")))))
    (:Completed
      ;[0.7715 1 0.7624] Puzzle completion
      (if (>= (Variables|Default|GetActivePlates) 3)
        (CallFunction|PuzzleComplete 1)))))

(fn ResetPuzzle2
  (Development|PrintString "Puzzle 2 reset." true true "(R=0.000000,G=0.660000,B=1.000000,A=1.000000)" 3.0 "P2Reset")
  (Utilities|Array|Clear (Variables|Default|GetPuzzle2PodiumsActivated))
  (Utilities|FlowControl|Sequence
    (:then_0
      ;[1 1 1] Reset cubes
      (bind _outactors (Actor|GetAllActorsOfClass "/Game/Blueprints/BP_Puzzle2Cube.BP_Puzzle2Cube_C"))
      (for _array_element _outactors
        (Default|PrimeforDrop _array_element)))
    (:then_1
      ;[1 1 1] Reset podium
      (bind _outactors_2 (Actor|GetAllActorsOfClass "/Game/Blueprints/BP_Puzzle2PodiumSpot.BP_Puzzle2PodiumSpot_C"))
      (for (_array_element_2 _array_index) _outactors_2
        (Default|DeactivatePodium _array_element_2)
        (if (== _array_index 0)
          (Audio|PlaySoundatLocation "/Game/Sound/PuzzleError_-_Universfield.PuzzleError_-_Universfield" (Transformation|GetWorldLocation (Variables|/Game/Blueprints/BP_Puzzle2PodiumSpot.BP_Puzzle2PodiumSpot_C|GetSM_PodiumSpot _array_element_2)) "0, 0, 0" 1.0 1.0 0.0 0 0 0 0)
          (Audio|PlaySoundatLocation "/Game/Sound/Puzzle2ResetWhoosh.Puzzle2ResetWhoosh" (Transformation|GetWorldLocation (Variables|/Game/Blueprints/BP_Puzzle2PodiumSpot.BP_Puzzle2PodiumSpot_C|GetSM_PodiumSpot _array_element_2)) "0, 0, 0" 1.2 1.0 0.05 0 0 0 0))))))

(fn EvaluatePuzzle2
  (params (PodiumID :type Integer))
  (bind _puzzle2podiumsactivated (Variables|Default|GetPuzzle2PodiumsActivated))
  ;[1 1 1] Add & organise progress
  (Utilities|Array|AddUnique _puzzle2podiumsactivated PodiumID)
  (Class|KismetArrayLibrary|SortIntArray _puzzle2podiumsactivated)
  ;[1 1 1] Check for #1 podium
  (if (== (Utilities|Array|Get(acopy) (Variables|Default|GetPuzzle2PodiumsActivated)) 1)
    ;[1 1 1] Is the player activating podiums in order?
    (bind _array_element (Utilities|Array|ForEachLoopwithBreak (Variables|Default|GetPuzzle2PodiumsActivated) :!label _label)
      (:LoopBody
        (if (== _array_element (LocalVariables|GetExpectedPodiumNumber))
          (Math|Integer|IncrementInt (LocalVariables|GetExpectedPodiumNumber) ; Check next Podium number
            (:%20%20
              (LocalVariables|SetProgressCorrect true)))
          (else
            (LocalVariables|SetProgressCorrect false) ; Puzzle failed
            (goto _label Break))))
      (:Completed
        (if (LocalVariables|GetProgressCorrect) ; If puzzle not failed?
          (if (>= (LocalVariables|GetExpectedPodiumNumber) (+ (Variables|Default|GetTotalPodiums) 1)) ; All podiums evaluated?
            ;[0 0.3115 0.06103] Puzzle complete
            (CallFunction|PuzzleComplete 2)
            (else
              ;[1 0.5214 0.1219] Prepare for next check
              (LocalVariables|SetExpectedPodiumNumber 1)))
          (else
            ;[0.2865 0 0] Puzzle reset
            (CallFunction|ResetPuzzle2 :!label _label_2)))))
    (else
      (goto _label_2))))