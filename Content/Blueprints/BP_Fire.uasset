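; BP_Fire is a fire actor with an Extinguish event that replaces the fire effect with steam.
; Extinguish starts a looping timer that, capped by a DoN, spawns two scaled-up steam particle systems at the root's location.
; Delayed steps then destroy the fire component and later the steam, with debug prints marking each stage.
; SpawnSteam overwrites its stored reference, so the cleanup destroys only the last steam component spawned.
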(event Custom|Extinguish
  (bind _cps_fire (Variables|Default|GetCPS_Fire))
  (Utilities|FlowControl|Sequence
    (:then_0
      ;[1 1 1] Steam while fire is extinguishing
      (Utilities|Time|SetTimerbyEvent (delegate Custom|SteamDuringExtinguish) 0.2 true)
      (Development|PrintString "Extinguish Pt. 1"))
    (:then_1
      (Utilities|FlowControl|Delay 2.0)
      ;[1 1 1] Destroys fire VFX component
      (if (Utilities|IsValid _cps_fire)
        (Components|DestroyComponent _cps_fire)
        (Development|PrintString "Extinguish Pt. 2")))
    (:then_2
      ;[1 1 1] Delete Steam
      (Utilities|Time|SetTimerbyEvent (delegate Custom|DeleteSteam) 5.0))))

(event Custom|DeleteSteam
  ;[1 1 1] Delete Steam
  (Components|DestroyComponent (Variables|Default|GetSteam%20Particle%20System%20Ref))
  (Development|PrintString "Extinguish Pt. 3"))

(event Custom|SteamDuringExtinguish
  ;[1 1 1] Steam while fire is extinguishing
  (bind _counter (Utilities|FlowControl|DoN 2)
    (:Exit
      (CallFunction|SpawnSteam)
      (Development|PrintString (Utilities|String|ToString(Integer) _counter)))))

(fn ConstructionScript)

(fn SpawnSteam
  ;[1 1 1] Spawns Steam
  (bind _returnvalue (AddComponent|AddParticleSystemComponent false))
  (bind _output_get (Variables|Default|SetSteam%20Particle%20System%20Ref _returnvalue))
  (Transformation|SetWorldLocation _output_get (Transformation|GetWorldLocation (Variables|Default|GetDefaultSceneRoot)) false true)
  (Transformation|SetWorldScale3D (Variables|Default|GetSteam%20Particle%20System%20Ref) "2.000000,2.000000,1.500000"))